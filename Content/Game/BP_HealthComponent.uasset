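; Health component that stores current and max health, with getters, setters and functions to add or remove health.
; Add and remove clamp health between zero and max, while the setters assign values unchecked.
; AddHealth calls a max-health event only when health is already full, and RemoveHealth calls a death event at zero.
; RemoveHealth prints debug messages and leaves its DamageCauser input unused.
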(event EventBeginPlay)

(event EventTick
  (params (DeltaSeconds :type Float%20%28single-precision%29)))

(fn GetHealth
  (return (Variables|Default|GetcurrentHealth)))

(fn GetMaxHealth
  (return (Variables|Default|GetmaxHealth)))

(fn SetHealth
  (params (NewCurrentHealth :type Float%20%28single-precision%29))
  (Variables|Default|SetcurrentHealth NewCurrentHealth))

(fn SetMaxHealth
  (params (NewMaxHealth :type Float%20%28single-precision%29))
  (Variables|Default|SetmaxHealth NewMaxHealth))

(fn AddHealth
  (params (addedHealth :type Float%20%28single-precision%29))
  (if (== (Variables|Default|GetmaxHealth) (Variables|Default|GetcurrentHealth))
    (Default|CallEventMaxHealth)
    (else
      (Variables|Default|SetcurrentHealth (Math|Float|Clamp(Float) (+ (Variables|Default|GetcurrentHealth) addedHealth) 0.0 (Variables|Default|GetmaxHealth))))))

(fn RemoveHealth
  (params (removedHealth :type Float%20%28single-precision%29) (DamageCauser :type Actor%20Object%20Reference))
  (bind _output_get (Variables|Default|SetcurrentHealth (Math|Float|Clamp(Float) (- (Variables|Default|GetcurrentHealth) removedHealth) 0.0 (Variables|Default|GetmaxHealth))))
  (if (== _output_get 0.0)
    (Default|CallEventDeath)
    (Development|PrintString "DEATH")
    (else
      (Development|PrintString (Utilities|String|Append "HEALTH IS NOW" (Utilities|String|ToString(Float) _output_get) " ") true true "(R=0.000000,G=0.675999,B=1.000000,A=1.000000)" 88.0))))