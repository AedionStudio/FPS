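; Player spawn point that flags whether it is free by watching for MyPlayer actors inside its DetectionRange.
; Shortly after BeginPlay, an initial overlap query sets IsAvailable without filling UserList.
; Begin and end overlaps then go through SRV-prefixed events that add or remove players in UserList.
; IsAvailable is recomputed whenever that list changes, false while any player is listed.
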(event OnComponentBeginOverlap(DetectionRange)
  (params (OverlappedComponent :type Primitive%20Component%20Object%20Reference) (OtherActor :type Actor%20Object%20Reference) (OtherComp :type Primitive%20Component%20Object%20Reference) (OtherBodyIndex :type Integer) (bFromSweep :type Boolean) (SweepResult :type Hit%20Result%20Structure%20%28by%20ref%29))
  (CallFunction|SRVOverlap OtherActor))

(event OnComponentEndOverlap(DetectionRange)
  (params (OverlappedComponent :type Primitive%20Component%20Object%20Reference) (OtherActor :type Actor%20Object%20Reference) (OtherComp :type Primitive%20Component%20Object%20Reference) (OtherBodyIndex :type Integer))
  (CallFunction|SRVEndOverlap OtherActor))

(event Custom|SRV_Overlap
  (params (OtherActor :type Actor%20Object%20Reference))
  (bind _userlist (Variables|Default|GetUserList))
  (Utilities|Casting|CastToMyPlayer OtherActor)
  (if (not (Utilities|Array|ContainsItem _userlist OtherActor))
    (Utilities|Array|Add _userlist OtherActor)
    (if (> (Utilities|Array|Length _userlist) 0)
      (Variables|Default|SetisAvailable false)
      (else
        (Variables|Default|SetisAvailable true)))))

(event Custom|SRV_EndOverlap
  (params (OtherActor :type Actor%20Object%20Reference))
  (bind _userlist (Variables|Default|GetUserList))
  (Utilities|Casting|CastToMyPlayer OtherActor)
  (if (Utilities|Array|ContainsItem _userlist OtherActor)
    (Utilities|Array|RemoveItem _userlist OtherActor)
    (if (> (Utilities|Array|Length _userlist) 0)
      (Variables|Default|SetisAvailable false)
      (else
        (Variables|Default|SetisAvailable true)))))

(event Custom|SRV_CheckOverlap
  (if (> (Utilities|Array|Length (Collision|GetOverlappingActors (Variables|Default|GetDetectionRange) "/Game/Game/MyPlayer.MyPlayer_C" :!class /Script/Engine.PrimitiveComponent)) 0)
    (Variables|Default|SetisAvailable false)
    (else
      (Variables|Default|SetisAvailable true))))

(event EventBeginPlay
  (Utilities|FlowControl|Delay 0.2)
  (CallFunction|SRVCheckOverlap))

(fn ConstructionScript)