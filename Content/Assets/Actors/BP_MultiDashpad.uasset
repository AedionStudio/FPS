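; BP_MultiDashpad is a dash pad that launches a Character along its arrow, changing direction after each use.
; A hit on the cube calls SRV_Overlap, which launches the Character with horizontal velocity overridden, then yaws the arrow 90 degrees.
; A DoOnce blocks relaunches during a two-second cooldown, while material swaps on the cube show the active or inactive state.
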(event OnComponentHit(Cube)
  (params (HitComponent :type Primitive%20Component%20Object%20Reference) (OtherActor :type Actor%20Object%20Reference) (OtherComp :type Primitive%20Component%20Object%20Reference) (NormalImpulse :type Vector :default "0, 0, 0") (Hit :type Hit%20Result%20Structure%20%28by%20ref%29))
  ;[1 1 1] Begin overlap myPlayer
  (CallFunction|SRVOverlap OtherActor))

(event Custom|Deactivate
  ;[1 1 1] Activate / Deactivate launchpad
  (Rendering|Material|SetMaterial (Variables|Default|GetCube) 0 "/Game/Assets/Material/DeActivate.Deactivate"))

(event Custom|Activate
  ;[1 1 1] Activate / Deactivate launchpad
  (Rendering|Material|SetMaterial (Variables|Default|GetCube) 0 "/Game/Assets/Material/Activate.Activate"))

(event Custom|AddArrowRotation
  ;[1 1 1] Rotate Arrow
  (Transformation|SetRelativeRotation (Variables|Default|GetArrow) (Math|Rotator|MakeRotator 0.0 0.0 (Variables|Default|Getrotation)) false false))

(event Custom|SRV_Overlap
  (params (OtherActor :type Actor%20Object%20Reference))
  ;[1 1 1] Begin overlap myPlayer
  (Utilities|FlowControl|DoOnce false :!label _label
    (:Completed
      (Character|LaunchCharacter (.AsCharacter (Utilities|Casting|CastToCharacter OtherActor)) (* (Math|Vector|GetForwardVector (Variables|Default|GetArrow)) 4e+03) true false)
      (CallFunction|Deactivate)
      (Variables|Default|Setrotation (+ (Variables|Default|Getrotation) 9e+01))
      (CallFunction|AddArrowRotation)
      (Utilities|FlowControl|Delay 2.0)
      (CallFunction|Activate)
      (goto _label Reset))))

(event EventBeginPlay
  ;[1 1 1] BeginPlay
  (CallFunction|Activate))

(fn ConstructionScript)