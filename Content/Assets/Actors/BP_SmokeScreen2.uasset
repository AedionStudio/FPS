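; Smoke screen actor that fades a post-process effect in while the player is inside its box volume.
; When MyPlayer begins overlapping, the FogIntensity timeline plays and drives the PostProcess blend weight; ending the overlap reverses it to fade the effect out.
; An older timer-based fade remains as custom events and disconnected nodes that never run.
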(event OnComponentBeginOverlap(Box)
  (params (OverlappedComponent :type Primitive%20Component%20Object%20Reference) (OtherActor :type Actor%20Object%20Reference) (OtherComp :type Primitive%20Component%20Object%20Reference) (OtherBodyIndex :type Integer) (bFromSweep :type Boolean) (SweepResult :type Hit%20Result%20Structure%20%28by%20ref%29))
  (Utilities|Casting|CastToMyPlayer OtherActor)
  (bind _weight (Timeline|FogIntensity Play)
    (:Update
      (Variables|/Script/Engine.PostProcessComponent|SetBlendWeight (Variables|Default|GetPostProcess) _weight))))

(event OnComponentEndOverlap(Box)
  (params (OverlappedComponent :type Primitive%20Component%20Object%20Reference) (OtherActor :type Actor%20Object%20Reference) (OtherComp :type Primitive%20Component%20Object%20Reference) (OtherBodyIndex :type Integer))
  (Utilities|Casting|CastToMyPlayer OtherActor)
  (bind _weight (Timeline|FogIntensity Reverse)
    (:Update
      (Variables|/Script/Engine.PostProcessComponent|SetBlendWeight (Variables|Default|GetPostProcess) _weight))))

(event Custom|CustomEvent
  (bind _postprocess (Variables|Default|GetPostProcess))
  (Variables|/Script/Engine.PostProcessComponent|SetBlendWeight _postprocess (- (Variables|/Script/Engine.PostProcessComponent|GetBlendWeight _postprocess) 0.1))
  (if (<= (- (Variables|/Script/Engine.PostProcessComponent|GetBlendWeight _postprocess) 0.1) -1.0)
    (Utilities|Time|ClearTimerbyFunctionName 0 "CustomEvent")))

(event Custom|CustomEvent_0)

(fn ConstructionScript)