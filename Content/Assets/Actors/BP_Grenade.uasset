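; BP_Grenade is a projectile grenade actor that explodes once it has slowed almost to a stop.
; On each Sphere hit it checks ProjectileMovement speed, and below a threshold waits briefly before applying radial damage with falloff at its location.
; It prints a debug "Boom" and destroys itself only if that damage call reports applying damage, so otherwise the actor remains in the world.
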(event OnComponentHit(Sphere)
  (params (HitComponent :type Primitive%20Component%20Object%20Reference) (OtherActor :type Actor%20Object%20Reference) (OtherComp :type Primitive%20Component%20Object%20Reference) (NormalImpulse :type Vector :default "0, 0, 0") (Hit :type Hit%20Result%20Structure%20%28by%20ref%29))
  (if (< (Math|Vector|VectorLength (Variables|/Script/Engine.MovementComponent|GetVelocity (Variables|Default|GetProjectileMovement))) 1e+02)
    (Utilities|FlowControl|Delay 0.2)
    (bind _returnvalue (Class|GameplayStatics|ApplyRadialDamagewithFalloff 5e+01 1e+01 (Transformation|GetActorLocation) 4.5e+02 9e+02 1.0 0 0 self 0 "ECC_Visibility"))
    (if _returnvalue
      (Development|PrintString "Boom")
      (Actor|DestroyActor))))

(fn ConstructionScript)