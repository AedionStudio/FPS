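; Launchpad actor that launches a MyPlayer character upward when it hits the pad, using a configurable strength.
; A component hit calls SRV_Overlap, which overrides the character's Z velocity and passes its unscaled forward vector as X and Y.
; A DoOnce gate blocks repeat launches until a cooldown delay resets it, while Activate and Deactivate swap the pad's material to show readiness.
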(event OnComponentHit(LaunchPad)
  (params (HitComponent :type Primitive%20Component%20Object%20Reference) (OtherActor :type Actor%20Object%20Reference) (OtherComp :type Primitive%20Component%20Object%20Reference) (NormalImpulse :type Vector :default "0, 0, 0") (Hit :type Hit%20Result%20Structure%20%28by%20ref%29))
  ;[1 1 1] Begin overlap myPlayer
  (CallFunction|SRVOverlap OtherActor))

(event Custom|Deactivate
  ;[1 1 1] Activate / Deactivate launchpad
  (Rendering|Material|SetMaterial (Variables|Default|GetLaunchPad) 0 "/Game/Assets/Material/DeActivate.Deactivate"))

(event Custom|Activate
  ;[1 1 1] Activate / Deactivate launchpad
  (Rendering|Material|SetMaterial (Variables|Default|GetLaunchPad) 0 "/Game/Assets/Material/Activate.Activate"))

(event Custom|SRV_Overlap
  (params (OtherActor :type Actor%20Object%20Reference))
  (bind _returnvalue (Transformation|GetActorForwardVector OtherActor))
  ;[1 1 1] Begin overlap myPlayer
  (bind _asmy_player (Utilities|Casting|CastToMyPlayer OtherActor))
  (Utilities|FlowControl|DoOnce false :!label _label
    (:Completed
      (Character|LaunchCharacter _asmy_player (Math|Vector|MakeVector (.x _returnvalue) (.y _returnvalue) (Variables|LaunchPad_Settings|GetLaunchpadStrength)) false true)
      (CallFunction|Deactivate)
      (Utilities|FlowControl|Delay (Variables|LaunchPad_Settings|GetCooldownTimer))
      (CallFunction|Activate)
      (goto _label Reset))))

(event EventBeginPlay
  ;[1 1 1] BeginPlay
  (CallFunction|Activate))

(fn ConstructionScript)