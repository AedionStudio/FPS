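; BP_MultiLaunchpad is a launch pad that throws the player along its arrow's horizontal direction with a fixed upward boost.
; A box overlap with MyPlayer passes a DoOnce gate, launches the character, then turns the arrow a quarter turn so successive launches cycle through directions.
; The cube's material shows the inactive state during a short delay, after which the pad reactivates and resets the gate.
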(event OnComponentBeginOverlap(Box)
  (params (OverlappedComponent :type Primitive%20Component%20Object%20Reference) (OtherActor :type Actor%20Object%20Reference) (OtherComp :type Primitive%20Component%20Object%20Reference) (OtherBodyIndex :type Integer) (bFromSweep :type Boolean) (SweepResult :type Hit%20Result%20Structure%20%28by%20ref%29))
  (bind _arrow (Variables|Default|GetArrow))
  (bind _returnvalue (Transformation|GetWorldRotation _arrow))
  (bind _returnvalue_2 (Math|Rotator|GetRotationXVector _returnvalue))
  ;[1 1 1] Begin overlap myPlayer
  (bind _asmy_player (Utilities|Casting|CastToMyPlayer OtherActor))
  (Utilities|FlowControl|DoOnce false :!label _label
    (:Completed
      (Character|LaunchCharacter _asmy_player (Math|Vector|MakeVector (* 2500 (.x _returnvalue_2)) (* 2500 (.y _returnvalue_2)) 9e+02) false false)
      (CallFunction|Deactivate)
      (CallFunction|AddArrowRotation)
      (Transformation|SetRelativeRotation (Variables|Default|GetArrow) (Math|Rotator|MakeRotator 0.0 0.0 (Variables|Default|Getrotation)) false false)
      (Utilities|FlowControl|Delay 2.0)
      (CallFunction|Activate)
      (goto _label Reset))))

(event Custom|Deactivate
  ;[1 1 1] Activate / Deactivate launchpad
  (Rendering|Material|SetMaterial (Variables|Default|GetCube) 0 "/Game/Assets/Material/DeActivate.Deactivate"))

(event Custom|Activate
  ;[1 1 1] Activate / Deactivate launchpad
  (Rendering|Material|SetMaterial (Variables|Default|GetCube) 0 "/Game/Assets/Material/Activate.Activate"))

(event Custom|AddArrowRotation
  ;[1 1 1] Rotate Arrow
  (Variables|Default|Setrotation (+ (Variables|Default|Getrotation) 9e+01)))

(event EventBeginPlay
  ;[1 1 1] BeginPlay
  (CallFunction|Activate))

(fn ConstructionScript)