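; BP_PositionSwitcher is a one-use trigger that swaps the positions and rotations of two players when a MyPlayer overlaps its collision.
; The overlap calls a SRV event, which takes the first other MyPlayer found, exchanges their transforms, then destroys the actor.
; An MC event sets each player's controller rotation to match the new facing.
; No check confirms that a second player was found before the swap.
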(event OnComponentBeginOverlap(Collision)
  (params (OverlappedComponent :type Primitive%20Component%20Object%20Reference) (OtherActor :type Actor%20Object%20Reference) (OtherComp :type Primitive%20Component%20Object%20Reference) (OtherBodyIndex :type Integer) (bFromSweep :type Boolean) (SweepResult :type Hit%20Result%20Structure%20%28by%20ref%29))
  (CallFunction|SRVOverlap OtherActor))

(event Custom|SRV_Overlap
  (params (OtherActor :type Actor%20Object%20Reference))
  (Utilities|FlowControl|DoOnce false
    (:Completed
      (bind _asmy_player (Utilities|Casting|CastToMyPlayer OtherActor))
      (bind _output_get (Variables|Default|SetAs%20My%20Player _asmy_player))
      (Variables|Default|SetMyPlayerTransform (Transformation|GetActorTransform _output_get))
      (bind _outactors (Actor|GetAllActorsOfClass "/Game/Game/MyPlayer.MyPlayer_C"))
      (bind _array_element (Utilities|Array|ForEachLoopwithBreak _outactors :!label _label)
        (:LoopBody
          (if (!= _array_element (Variables|Default|GetAs%20My%20Player))
            (Variables|Default|SetAsOtherPlayer _array_element)
            (goto _label Break)))
        (:Completed
          (Utilities|IsValid (Variables|Default|GetAs%20My%20Player)
            (:Is%20Valid
              (Transformation|SetActorLocationAndRotation (Variables|Default|GetAs%20My%20Player) (.location (Transformation|GetActorTransform (Variables|Default|GetAsOtherPlayer))) (.rotation (Transformation|GetActorTransform (Variables|Default|GetAsOtherPlayer))))
              (CallFunction|MCSetRotation (Variables|Default|GetAs%20My%20Player) (.rotation (Transformation|GetActorTransform (Variables|Default|GetAsOtherPlayer))))
              (Transformation|SetActorLocationAndRotation (Variables|Default|GetAsOtherPlayer) (.Location (Math|Transform|BreakTransform (Variables|Default|GetMyPlayerTransform))) (.Rotation (Math|Transform|BreakTransform (Variables|Default|GetMyPlayerTransform))))
              (CallFunction|MCSetRotation (Variables|Default|GetAsOtherPlayer) (.Rotation (Math|Transform|BreakTransform (Variables|Default|GetMyPlayerTransform))))
              (Actor|DestroyActor))
            (:Is%20Not%20Valid
              (Development|PrintString "No Player Found" true true "(R=1.000000,G=0.014920,B=0.000000,A=1.000000)" 8.0))))))))

(event Custom|MC_SetRotation
  (params (NewParam :type Actor%20Object%20Reference) (NewParam2 :type Rotator))
  (bind _asmy_player (Utilities|Casting|CastToMyPlayer NewParam))
  (Utilities|IsValid (Pawn|GetController _asmy_player)
    (:Is%20Valid
      (Pawn|SetControlRotation (Pawn|GetController _asmy_player) NewParam2))))

(fn ConstructionScript)