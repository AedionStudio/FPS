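; Grenade projectile that explodes after it settles from bouncing, damaging and shaking cameras around it.
; A bounce below a small impact speed starts a fuse delay, then applies radial damage with falloff and a camera shake over matching radii before destroying the actor.
; A separate lifetime timer from BeginPlay destroys it with only a debug "Boom" print, without damage or shake.
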(event OnProjectileBounce(ProjectileMovement)
  (params (ImpactResult :type Hit%20Result%20Structure%20%28by%20ref%29) (ImpactVelocity :type Vector%20%28by%20ref%29 :default "0, 0, 0"))
  (if (< (Math|Vector|VectorLength ImpactVelocity) 1e+02)
    (Utilities|FlowControl|Delay 3.0)
    (bind _returnvalue (Class|GameplayStatics|ApplyRadialDamagewithFalloff 5e+01 1e+01 (Transformation|GetActorLocation) 4.5e+02 9e+02 1.0 0 0 self 0 "ECC_Visibility"))
    (if _returnvalue
      _
      (else
        _))
    (Development|PrintString "Boom" true true "(R=1.000000,G=0.000000,B=0.070089,A=1.000000)")
    (Camera|PlayWorldCameraShake "/Game/Assets/Actors/Projectiles/BP_CameraShake.BP_CameraShake_C" (Transformation|GetActorLocation) 4.5e+02 9e+02)
    (Actor|DestroyActor)))

(event EventBeginPlay
  (Utilities|FlowControl|Delay 1e+01)
  (Development|PrintString "Boom")
  (Actor|DestroyActor))

(fn ConstructionScript)