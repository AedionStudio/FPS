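; Dash pad actor that launches any Character hitting it along that character's control rotation forward vector, scaled by DashStrength.
; The DashPad component's hit event feeds SRV_Overlap, which calls LaunchCharacter, overriding XY velocity and adding to Z.
; A DoOnce gate blocks retriggering until a CooldownTimer delay ends and resets it.
; Activate and Deactivate swap the pad's material to show whether it is ready.
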(event OnComponentHit(DashPad)
  (params (HitComponent :type Primitive%20Component%20Object%20Reference) (OtherActor :type Actor%20Object%20Reference) (OtherComp :type Primitive%20Component%20Object%20Reference) (NormalImpulse :type Vector :default "0, 0, 0") (Hit :type Hit%20Result%20Structure%20%28by%20ref%29))
  ;[1 1 1] Begin overlap myPlayer
  (CallFunction|SRVOverlap OtherActor))

(event Custom|Deactivate
  ;[1 1 1] Activate / Deactivate launchpad
  (Rendering|Material|SetMaterial (Variables|Default|GetDashPad) 0 "/Game/Assets/Material/DeActivate.Deactivate"))

(event Custom|Activate
  ;[1 1 1] Activate / Deactivate launchpad
  (Rendering|Material|SetMaterial (Variables|Default|GetDashPad) 0 "/Game/Assets/Material/Activate.Activate"))

(event Custom|SRV_Overlap
  (params (OtherActor :type Actor%20Object%20Reference))
  ;[1 1 1] Begin overlap myPlayer
  (bind _ascharacter (Utilities|Casting|CastToCharacter OtherActor))
  (Utilities|FlowControl|DoOnce false :!label _label
    (:Completed
      (Character|LaunchCharacter _ascharacter (* (Math|Rotator|GetRotationXVector (Pawn|GetControlRotation _ascharacter :!class /Script/Engine.Pawn)) (Variables|DashPad_Settings|GetDashStrength)) true false)
      (CallFunction|Deactivate)
      (Utilities|FlowControl|Delay (Variables|DashPad_Settings|GetCooldownTimer))
      (CallFunction|Activate)
      (goto _label Reset))))

(event EventBeginPlay
  ;[1 1 1] BeginPlay
  (CallFunction|Activate))

(fn ConstructionScript)