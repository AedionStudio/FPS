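; Assault rifle weapon Blueprint that fires hitscan shots and tracks its ammo count.
; The left-mouse action gets trace endpoints from the player and passes them to the SRV_Fire event, which decrements ammo or calls Discard when empty.
; That event runs a debug-drawn complex line trace on the Camera channel, ignoring the shooter, and applies fixed damage to the hit actor.
; Getters expose current and maximum ammo.
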(event Custom|SRV_Fire
  (params (Start :type Vector) (End :type Vector) (NewParam :type My%20Player%20Object%20Reference))
  (if (== (Variables|Default|GetcurrentAmmo) 0)
    (CallFunction|Discard)
    (else
      (Variables|Default|SetcurrentAmmo (- (Variables|Default|GetcurrentAmmo) 1))))
  (bind (_outhit _returnvalue) (Collision|LineTraceByChannel Start End "TraceTypeQuery2" true (Utilities|Array|MakeArray NewParam) "ForDuration"))
  (if _returnvalue
    (Game|Damage|ApplyDamage (.HitActor (Collision|BreakHitResult _outhit)) 75.0 0 0)))

(event EventLMBAction
  (params (MyPlayer :type Character%20Object%20Reference))
  (bind (_start _end _player) (CallFunction|GetLinetraceLocation MyPlayer))
  (CallFunction|SRVFire _start _end _player))

(fn ConstructionScript
  (|CallParentFunction))

(fn GetMaxAmmo
  (return (Variables|Default|GetmaxAmmo)))

(fn GetAmmo
  (return (Variables|Default|GetcurrentAmmo)))