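; BP_GranadeLauncher is a grenade launcher weapon that fires BP_Grenade actors.
; LMBAction gets a line trace start point and passes it with the player's control rotation to SRV_Fire, a server-style event.
; SRV_Fire decrements ammo, then either spawns the grenade there or, at zero, discards the weapon without spawning one.
; Two getters expose current and maximum ammo.
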(event Custom|SRV_Fire
  (params (Start :type Vector) (End :type Vector) (MyPlayer :type My%20Player%20Object%20Reference) (NewParam :type Rotator))
  (bind _output_get (Variables|Default|SetcurrentAmmo (- (Variables|Default|GetcurrentAmmo) 1)))
  (if (== _output_get 0)
    (CallFunction|Discard)
    (else
      (Game|SpawnActorfromClass "/Game/Assets/Actors/Projectiles/BP_Grenade.BP_Grenade_C" (Math|Transform|MakeTransform Start NewParam "1,1,1") "AdjustIfPossibleButAlwaysSpawn" 0 0))))

(event EventLMBAction
  (params (MyPlayer :type Character%20Object%20Reference))
  (bind (_start _end _player) (CallFunction|GetLinetraceLocation MyPlayer))
  (CallFunction|SRVFire _start _end _player (Pawn|GetControlRotation _player :!class /Script/Engine.Pawn)))

(fn ConstructionScript
  (|CallParentFunction))

(fn GetMaxAmmo
  (return (Variables|Default|GetmaxAmmo)))

(fn GetAmmo
  (return (Variables|Default|GetcurrentAmmo)))