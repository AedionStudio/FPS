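; Automatic rifle weapon Blueprint that fires hitscan shots for the player and toggles an aim zoom.
; LMBAction starts a looping timer that line-traces on the Camera channel and applies damage to the hit actor.
; RMBAction flip-flops between the player's normal and zoom cameras, adjusting mouse sensitivity.
; Timer clearing and ammo consumption are unwired, so LMBRelease does nothing and firing never stops or uses ammo.
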(event Custom|ShootAutomaticRifle
  (bind _outhit (Collision|LineTraceByChannel (stale EventLMBAction Start) (stale EventLMBAction End) "TraceTypeQuery2" true (Utilities|Array|MakeArray (stale EventLMBAction _asmy_player)) "ForDuration"))
  (Game|Damage|ApplyDamage (.HitActor (Collision|BreakHitResult _outhit)) 8.0 0 0))

(event EventBeginPlay
  (|CallParentFunction))

(event Collision|EventActorBeginOverlap
  (params (OtherActor :type Actor%20Object%20Reference))
  (|CallParentFunction OtherActor))

(event EventTick
  (params (DeltaSeconds :type Float%20%28single-precision%29))
  (|CallParentFunction DeltaSeconds))

(event EventLMBAction
  (params (Start :type Vector :default "0, 0, 0") (End :type Vector :default "0, 0, 0") (MyPlayer :type Character%20Object%20Reference))
  (bind _asmy_player (Utilities|Casting|CastToMyPlayer MyPlayer))
  (Utilities|Time|SetTimerbyFunctionName 0 "ShootAutomaticRifle" 0.1 true))

(event EventRMBAction
  (params (MyPlayer :type Character%20Object%20Reference))
  (bind _asmy_player (Utilities|Casting|CastToMyPlayer MyPlayer))
  (bind _output_get (Variables|Default|SetAs%20My%20Player _asmy_player))
  (Utilities|FlowControl|FlipFlop
    (:A
      (Components|Activation|SetActive (Variables|/Game/Game/MyPlayer.MyPlayer_C|GetCamera _output_get) false false)
      (Components|Activation|SetActive (Variables|/Game/Game/MyPlayer.MyPlayer_C|Getzoomcam _output_get) true false)
      (Variables|/Game/Game/MyPlayer.MyPlayer_C|SetMouseSensitivity _output_get 15.0))
    (:B
      (Components|Activation|SetActive (Variables|/Game/Game/MyPlayer.MyPlayer_C|GetCamera _output_get) true false)
      (Components|Activation|SetActive (Variables|/Game/Game/MyPlayer.MyPlayer_C|Getzoomcam _output_get) false false)
      (Variables|/Game/Game/MyPlayer.MyPlayer_C|SetMouseSensitivity _output_get 3e+01))))

(event EventLMBRelease)

(event Input|AxisEvents|InputAxisTurn
  (params (AxisValue :type Float%20%28single-precision%29))
  (Pawn|Input|AddControllerYawInput (Variables|Default|GetAs%20My%20Player) AxisValue))

(event Input|AxisEvents|InputAxisLookUp
  (params (AxisValue :type Float%20%28single-precision%29))
  (Pawn|Input|AddControllerPitchInput (Variables|Default|GetAs%20My%20Player) AxisValue))

(fn ConstructionScript
  (|CallParentFunction))

(fn GetMaxAmmo
  (return (Variables|Default|GetmaxAmmo)))

(fn GetAmmo
  (return (Variables|Default|GetcurrentAmmo)))