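; Weapon helper library with functions to throw away a held weapon and to compute aim trace endpoints for MyPlayer.
; DiscardWeapon detaches the weapon, turns its static mesh into a blocking physics body, launches it along the owner's control rotation and clears the player's WeaponActor.
; GetLinetraceLocation returns start and end points along the player camera's forward vector, plus the cast player, without performing the trace.
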(fn DiscardWeapon
  (params (DiscardedWeapon :type Actor%20Object%20Reference))
  (bind _returnvalue (Actor|GetComponentbyClass DiscardedWeapon "/Script/Engine.StaticMeshComponent"))
  (bind _returnvalue_2 (Components|GetOwner DiscardedWeapon))
  (Utilities|IsValid DiscardedWeapon
    (:Is%20Valid
      (Transformation|DetachFromActor DiscardedWeapon "KeepWorld" "KeepWorld" "KeepWorld")
      (Collision|SetCollisionProfileName _returnvalue "BlockAll" true :!class /Script/Engine.PrimitiveComponent)
      (Physics|SetSimulatePhysics _returnvalue true)
      (Physics|AddImpulse _returnvalue (* (Math|Rotator|GetRotationXVector (Pawn|GetControlRotation (Variables|/Script/Engine.Actor|GetInstigator _returnvalue_2) :!class /Script/Engine.Pawn)) 2e+03) "None" true)
      (Variables|/Game/Game/MyPlayer.MyPlayer_C|SetWeaponActor (.AsMy%20Player (Utilities|Casting|CastToMyPlayer _returnvalue_2)) 0))))

(fn GetLinetraceLocation
  (params (MyPlayer :type Character%20Object%20Reference))
  (bind _asmy_player (Utilities|Casting|CastToMyPlayer MyPlayer))
  (return (Transformation|GetWorldLocation (Variables|/Game/Game/MyPlayer.MyPlayer_C|GetCamera _asmy_player)) (+ (* (Math|Vector|GetForwardVector (Variables|/Game/Game/MyPlayer.MyPlayer_C|GetCamera _asmy_player)) (LocalVariables|GetTracelength)) (Transformation|GetWorldLocation (Variables|/Game/Game/MyPlayer.MyPlayer_C|GetCamera _asmy_player))) _asmy_player))