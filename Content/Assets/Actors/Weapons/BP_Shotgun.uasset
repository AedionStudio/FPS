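; Shotgun weapon Blueprint with spread hitscan fire, an ammo count and a toggled zoom.
; LMBAction runs two passes, each spending one ammo and either discarding at zero or line-tracing with random end offset.
; Hits apply damage equal to the dot product of trace start and impact point, then print it.
; RMBAction flip-flops the player's cameras and mouse sensitivity; Turn and LookUp axes drive that cached player's view.
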(event EventBeginPlay
  (|CallParentFunction))

(event Collision|EventActorBeginOverlap
  (params (OtherActor :type Actor%20Object%20Reference))
  (|CallParentFunction OtherActor))

(event EventTick
  (params (DeltaSeconds :type Float%20%28single-precision%29))
  (|CallParentFunction DeltaSeconds))

(event EventLMBAction
  (params (Start :type Vector :default "0, 0, 0") (End :type Vector :default "0, 0, 0") (MyPlayer :type Character%20Object%20Reference))
  (for _index (range 0 1)
    (bind _asmy_player (Utilities|Casting|CastToMyPlayer MyPlayer))
    (bind _output_get (Variables|Default|SetAs%20My%20Player _asmy_player))
    (Utilities|IsValid _output_get
      (:Is%20Valid
        (bind _output_get_2 (Variables|Default|SetcurrentAmmo (- (Variables|Default|GetcurrentAmmo) 1)))
        (if (== _output_get_2 0)
          (CallFunction|Discard)
          (else
            (bind (_outhit _returnvalue) (Collision|LineTraceByChannel Start (+ End (Math|Vector|MakeVector (Math|Random|RandomFloatinRange -4e+02 4e+02) (Math|Random|RandomFloatinRange -4e+02 4e+02) (Math|Random|RandomFloatinRange -4e+02 4e+02))) "TraceTypeQuery1" true (Utilities|Array|MakeArray (Variables|Default|GetAs%20My%20Player)) "ForDuration"))
            (if _returnvalue
              (bind _returnvalue_2 (Game|Damage|ApplyDamage (.HitActor (Collision|BreakHitResult _outhit)) (Math|Vector|DotProduct (.TraceStart (Collision|BreakHitResult _outhit)) (.ImpactPoint (Collision|BreakHitResult _outhit))) 0 0))
              (Development|PrintString (Utilities|String|ToString(Float) _returnvalue_2)))))))))

(event EventRMBAction
  (params (MyPlayer :type Character%20Object%20Reference))
  (bind _asmy_player (Utilities|Casting|CastToMyPlayer MyPlayer))
  (bind _output_get (Variables|Default|SetAs%20My%20Player _asmy_player))
  (Utilities|FlowControl|FlipFlop
    (:A
      (Components|Activation|SetActive (Variables|/Game/Game/MyPlayer.MyPlayer_C|GetCamera _output_get) false false)
      (Components|Activation|SetActive (Variables|/Game/Game/MyPlayer.MyPlayer_C|Getzoomcam _output_get) true false)
      (Variables|/Game/Game/MyPlayer.MyPlayer_C|SetMouseSensitivity _output_get 15.0))
    (:B
      (Components|Activation|SetActive (Variables|/Game/Game/MyPlayer.MyPlayer_C|GetCamera _output_get) true false)
      (Components|Activation|SetActive (Variables|/Game/Game/MyPlayer.MyPlayer_C|Getzoomcam _output_get) false false)
      (Variables|/Game/Game/MyPlayer.MyPlayer_C|SetMouseSensitivity _output_get 3e+01))))

(event Input|AxisEvents|InputAxisTurn
  (params (AxisValue :type Float%20%28single-precision%29))
  (Pawn|Input|AddControllerYawInput (Variables|Default|GetAs%20My%20Player) AxisValue))

(event Input|AxisEvents|InputAxisLookUp
  (params (AxisValue :type Float%20%28single-precision%29))
  (Pawn|Input|AddControllerPitchInput (Variables|Default|GetAs%20My%20Player) AxisValue))

(fn ConstructionScript
  (|CallParentFunction))

(fn GetMaxAmmo
  (return (Variables|Default|GetmaxAmmo)))

(fn GetAmmo
  (return (Variables|Default|GetcurrentAmmo)))