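; Turret actor that tracks the player inside its DetectionSphere and repeatedly triggers a Shoot event.
; Sphere overlaps, plus a delayed check at BeginPlay, store the player and toggle a fast looping LookToPlayer timer.
; That timer sets the Arrow's relative rotation from LookAt and drives a Delay-paced firing loop while active.
; Shoot is an empty event here, so no firing logic is implemented in this Blueprint.
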(event OnComponentBeginOverlap(DetectionSphere)
  (params (OverlappedComponent :type Primitive%20Component%20Object%20Reference) (OtherActor :type Actor%20Object%20Reference) (OtherComp :type Primitive%20Component%20Object%20Reference) (OtherBodyIndex :type Integer) (bFromSweep :type Boolean) (SweepResult :type Hit%20Result%20Structure%20%28by%20ref%29))
  (bind _asmy_player (Utilities|Casting|CastToMyPlayer OtherActor))
  (Variables|Default|SetMyPlayer _asmy_player)
  (Utilities|Time|SetTimerbyFunctionName 0 "LookToPlayer" 0.001 true)
  (Variables|Default|SetisActive true))

(event OnComponentEndOverlap(DetectionSphere)
  (params (OverlappedComponent :type Primitive%20Component%20Object%20Reference) (OtherActor :type Actor%20Object%20Reference) (OtherComp :type Primitive%20Component%20Object%20Reference) (OtherBodyIndex :type Integer))
  (Utilities|Casting|CastToMyPlayer OtherActor)
  (Utilities|Time|ClearTimerbyFunctionName 0 "LookToPlayer")
  (Variables|Default|SetisActive false))

(event Custom|LookToPlayer
  (Transformation|SetRelativeRotation (Variables|Default|GetArrow) (CallFunction|Lookat) false false)
  (if (Variables|Default|GetisActive) :!label _label
    (Utilities|FlowControl|Delay 2.0)
    (CallFunction|Shoot)
    (goto _label)))

(event Custom|Shoot)

(event EventBeginPlay
  (bind _detectionsphere (Variables|Default|GetDetectionSphere))
  (bind _overlappingactors (Collision|GetOverlappingActors _detectionsphere "/Game/Game/MyPlayer.MyPlayer_C" :!class /Script/Engine.PrimitiveComponent))
  (Utilities|FlowControl|Delay 0.5)
  (if (> (Utilities|Array|Length _overlappingactors) 0)
    (bind _asmy_player (Utilities|Casting|CastToMyPlayer (Utilities|Array|Get(acopy) _overlappingactors)))
    (Variables|Default|SetMyPlayer _asmy_player)
    (Utilities|Time|SetTimerbyFunctionName 0 "LookToPlayer" 0.001 true)
    (Variables|Default|SetisActive true)))

(fn ConstructionScript)

(fn Lookat
  (return (Math|Rotator|FindLookatRotation (Transformation|GetActorLocation) (Transformation|GetActorLocation (Variables|Default|GetMyPlayer)))))